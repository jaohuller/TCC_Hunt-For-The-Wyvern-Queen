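; BP_BigFireball is a fireball hazard that damages BP_Khorvill on overlap.
; On BeginPlay it plays attached sound and Niagara, zeroes the projectile's gravity and velocity, and self-destructs after a short delay.
; A vulnerable Khorvill overlapping the sphere catches fire and triggers an explosion actor and sound.
; A DoOnce-gated interface message applies damage credited to the first BP_Fulghorra_02 found, then the fireball destroys itself.
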(event OnComponentBeginOverlap(Sphere)
  (params (OverlappedComponent :type Primitive%20Component%20Object%20Reference) (OtherActor :type Actor%20Object%20Reference) (OtherComp :type Primitive%20Component%20Object%20Reference) (OtherBodyIndex :type Integer) (bFromSweep :type Boolean) (SweepResult :type Hit%20Result%20Structure%20%28by%20ref%29))
  (bind _asbp_khorvill (Utilities|Casting|CastToBP_Khorvill OtherActor))
  (Utilities|IsValid _asbp_khorvill
    (:Is%20Valid
      (if (not (Variables|/Game/MyGame/Characters/01_Khorvill/BP_Khorvill.BP_Khorvill_C|GetisInvulnerable? _asbp_khorvill))
        (Default|OnFireEvent _asbp_khorvill)
        (bind _outactors (Actor|GetAllActorsOfClass "/Game/MyGame/Characters/Fulghorra/BP_Fulghorra_02.BP_Fulghorra_02_C"))
        (Audio|PlaySoundatLocation "/Game/MyGame/Sounds/KhorvillSounds/Cues/explosion_Cue.explosion_Cue" (Transformation|GetWorldLocation (Variables|/Script/Engine.Character|GetCapsuleComponent _asbp_khorvill)) "0, 0, 0" 1.0 1.0 0.0 0 0 0 0)
        (Game|SpawnActorfromClass "/Game/MyGame/VFX/BP_Explosion.BP_Explosion_C" (Math|Transform|MakeTransform (Transformation|GetWorldLocation (Variables|/Script/Engine.Character|GetCapsuleComponent _asbp_khorvill)) "0, 0, 0" "1.000000,1.000000,1.000000") "Undefined" 0 0)
        (Utilities|FlowControl|DoOnce false :!label _label
          (:Completed
            (Class|BPICombat|INTHitHandle(Message) _asbp_khorvill (Utilities|Array|Get(acopy) _outactors) 5e+01 (Variables|Default|GetAdditional%20Info))
            (Actor|DestroyActor)
            (Utilities|FlowControl|Delay 5.0)
            (goto _label Reset)))))))

(event EventBeginPlay
  (bind _projectilemovement (Variables|Default|GetProjectileMovement))
  (Audio|SpawnSoundAttached "/Game/MyGame/Sounds/KhorvillSounds/Cues/OnFireFireball_Cue.OnFireFireball_Cue" (Variables|Default|GetSphere) "None" "0, 0, 0" "0, 0, 0" "KeepRelativeOffset" false 1.0 1.0 0.0 0 0)
  (Components|Activation|SetActive (Variables|Default|GetNS_BigFireball) true false)
  (Variables|/Script/Engine.ProjectileMovementComponent|SetProjectileGravityScale _projectilemovement 0.0)
  (Variables|/Script/Engine.MovementComponent|SetVelocity _projectilemovement "0, 0, 0")
  (Utilities|FlowControl|Delay 5.0)
  (Actor|DestroyActor))

(fn ConstructionScript)